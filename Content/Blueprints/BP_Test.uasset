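; BP_Test is a debug actor for exercising the Gameplay Ability System and inventory system.
; Its Box applies GE_Test to overlapping Player-tagged actors, and an attribute-change delegate, bound a tick after BeginPlay, prints a player attribute.
; Debug keys add or remove test items.
; Input enabling and the item-change print binding are disconnected, so neither runs.
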(event OnComponentBeginOverlap(Box)
  (params (OverlappedComponent :type Primitive%20Component%20Object%20Reference) (OtherActor :type Actor%20Object%20Reference) (OtherComp :type Primitive%20Component%20Object%20Reference) (OtherBodyIndex :type Integer) (bFromSweep :type Boolean) (SweepResult :type Hit%20Result%20Structure%20%28by%20ref%29))
  (bind _returnvalue (Ability|GetAbilitySystemComponent OtherActor))
  (if (and (Actor|ActorHasTag OtherActor "Player") (Utilities|IsValid _returnvalue))
    (GameplayEffects|ApplyGameplayEffectToSelf :self _returnvalue :GameplayEffectClass "/Game/Blueprints/GAS/Effect/GE_Test.GE_Test_C")))

(event Custom|OnItemChange
  (params (ItemID :type Integer))
  (Development|PrintString (Utilities|String|Append (Utilities|String|ToString(Integer) ItemID) (Utilities|String|ToString(Integer) (Class|InventorySystem|GetItemNum (Subsystems|GetInventorySystem) ItemID)))))

(event Custom|AttrChange
  (Development|PrintString (Utilities|String|ToString(Float) (.ReturnValue (Ability|Attribute|GetFloatAttributefromAbilitySystemComponent (Ability|GetAbilitySystemComponent (stale EventBeginPlay _returnvalue)) "(AttributeName=\"Health\",Attribute=/Script/UECRPG.BasicAttributeSet:Health,AttributeOwner=\"/Script/CoreUObject.Class'/Script/UECRPG.BasicAttributeSet'\")")))))

(event EventBeginPlay
  (Utilities|FlowControl|DelayUntilNextTick)
  (bind _returnvalue (Class|GlobalFunc|GetPlayer))
  (EventDispatchers|BindEventtoOnAttributeChangeDelegate (Class|CharacterBase|GetCharacterHandleComponent _returnvalue) (delegate Custom|AttrChange)))

(event Input|KeyboardEvents|DebugKeyA
  (params (Key :type Key%20Structure :default "None") (ActionValue :type Input%20Action%20Value%20Structure))
  (:Pressed
    (Class|InventorySystem|AddItem (Subsystems|GetInventorySystem) 1001 2 true)))

(event Input|KeyboardEvents|DebugKeyD
  (params (Key :type Key%20Structure :default "None") (ActionValue :type Input%20Action%20Value%20Structure))
  (:Pressed
    (Class|InventorySystem|ReduceItem (Subsystems|GetInventorySystem) 1001 2 true)))

(event Input|KeyboardEvents|DebugKeyT
  (params (Key :type Key%20Structure :default "None") (ActionValue :type Input%20Action%20Value%20Structure))
  (:Pressed
    (Class|InventorySystem|AddItem (Subsystems|GetInventorySystem) 1002 2 true)))

(fn ConstructionScript)